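; BP_Hammer is a hammer pickup that the first-person character collects into inventory slot 1.
; A Sphere overlap enables input and shows the HammerHud widget, both reverted on exit.
; CollectBox overlap binds Collect to the character's CollectItem event.
; Collect plays a sound, then claims an empty slot or stacks onto existing hammers and destroys the actor; a slot holding another item leaves it in place.
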(event `self.Sphere.OnComponentBeginOverlap`
  (params (OverlappedComponent :type "PrimitiveComponent Object Reference") (OtherActor :type "Actor Object Reference") (OtherComp :type "PrimitiveComponent Object Reference") (OtherBodyIndex :type Integer) (bFromSweep :type Boolean) (SweepResult :type "HitResult Structure (by ref)"))
  (cast `/Game/FirstPerson/Blueprints/BP_FirstPersonCharacter` OtherActor)
  (`self.EnableInput` (`GameplayStatics.GetPlayerController` 0))
  (bind _returnvalue (`|GenericCreateObject` "/Game/1-TimeIsOut/Hammer/HammerHud.HammerHud_C"))
  (`UserWidget.AddToViewport` _returnvalue 0))

(event `self.Sphere.OnComponentEndOverlap`
  (params (OverlappedComponent :type "PrimitiveComponent Object Reference") (OtherActor :type "Actor Object Reference") (OtherComp :type "PrimitiveComponent Object Reference") (OtherBodyIndex :type Integer))
  (cast `/Game/FirstPerson/Blueprints/BP_FirstPersonCharacter` OtherActor)
  (`self.DisableInput` (`GameplayStatics.GetPlayerController` 0))
  (`Widget.RemoveFromParent` (stale `self.Sphere.OnComponentBeginOverlap` _returnvalue)))

(event `Collect`
  (`GameplayStatics.PlaySound2D` "/Game/1-TimeIsOut/Sounds/Hammer-Pickup.Hammer-Pickup" 1.0 1.0 0.0 null null)
  (if (`/Game/FirstPerson/Blueprints/BP_FirstPersonCharacter.Slot1INV` (stale `self.CollectBox.OnComponentBeginOverlap` _asbp_first_person_character))
    (if (== (`/Game/FirstPerson/Blueprints/BP_FirstPersonCharacter.Slot1IMG` (stale `self.CollectBox.OnComponentBeginOverlap` _asbp_first_person_character)) 1)
      (set `/Game/FirstPerson/Blueprints/BP_FirstPersonCharacter.Hammer` (+ (`/Game/FirstPerson/Blueprints/BP_FirstPersonCharacter.Hammer` (stale `self.CollectBox.OnComponentBeginOverlap` _asbp_first_person_character)) 1.0) (stale `self.CollectBox.OnComponentBeginOverlap` _asbp_first_person_character))
      (set `/Game/FirstPerson/Blueprints/BP_FirstPersonCharacter.Slot1` (+ (`/Game/FirstPerson/Blueprints/BP_FirstPersonCharacter.Slot1` (stale `self.CollectBox.OnComponentBeginOverlap` _asbp_first_person_character)) 1) (stale `self.CollectBox.OnComponentBeginOverlap` _asbp_first_person_character))
      (`self.K2_DestroyActor`))
    (else
      (set `/Game/FirstPerson/Blueprints/BP_FirstPersonCharacter.Slot1IMG` 1 (stale `self.CollectBox.OnComponentBeginOverlap` _asbp_first_person_character))
      (set `/Game/FirstPerson/Blueprints/BP_FirstPersonCharacter.Hammer` (+ (`/Game/FirstPerson/Blueprints/BP_FirstPersonCharacter.Hammer` (stale `self.CollectBox.OnComponentBeginOverlap` _asbp_first_person_character)) 1.0) (stale `self.CollectBox.OnComponentBeginOverlap` _asbp_first_person_character))
      (set `/Game/FirstPerson/Blueprints/BP_FirstPersonCharacter.Slot1` (+ (`/Game/FirstPerson/Blueprints/BP_FirstPersonCharacter.Slot1` (stale `self.CollectBox.OnComponentBeginOverlap` _asbp_first_person_character)) 1) (stale `self.CollectBox.OnComponentBeginOverlap` _asbp_first_person_character))
      (set `/Game/FirstPerson/Blueprints/BP_FirstPersonCharacter.Slot1INV` true (stale `self.CollectBox.OnComponentBeginOverlap` _asbp_first_person_character))
      (`self.K2_DestroyActor`))))

(event `self.CollectBox.OnComponentBeginOverlap`
  (params (OverlappedComponent :type "PrimitiveComponent Object Reference") (OtherActor :type "Actor Object Reference") (OtherComp :type "PrimitiveComponent Object Reference") (OtherBodyIndex :type Integer) (bFromSweep :type Boolean) (SweepResult :type "HitResult Structure (by ref)"))
  (bind _asbp_first_person_character (cast `/Game/FirstPerson/Blueprints/BP_FirstPersonCharacter` OtherActor))
  (add `/Game/FirstPerson/Blueprints/BP_FirstPersonCharacter.CollectItem` _asbp_first_person_character (delegate `Collect`)))

(fn `UserConstructionScript`)